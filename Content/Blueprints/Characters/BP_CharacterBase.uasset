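; Base character Blueprint that uses the Gameplay Ability System for melee combat.
; It acquires GA_Melee on BeginPlay and tries to activate it by class through the MeleeAttack event.
; Sword collider overlaps with exact-class BP_Enemy actors send the character a deal-damage gameplay event carrying the enemy as target.
; Tick prints current health from the attribute set as debug output.
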(event `self.ReceiveBeginPlay`
  (`self.AcquireAbility` "/Game/Blueprints/Characters/GameplayAbilities/Melee/GA_Melee.GA_Melee_C"))

(event `MeleeAttack`
  (`AbilitySystemComponent.TryActivateAbilityByClass` (`self.AbilitySystemComp`) "/Game/Blueprints/Characters/GameplayAbilities/Melee/GA_Melee.GA_Melee_C" true))

(event `self.ReceiveTick`
  (params (DeltaSeconds :type "Float (single-precision)"))
  (bind (_health_basevalue _health_currentvalue) (break `GameplayAttributeData` (`AttributeSetBase.Health` (`self.AttributeSetBaseComp`))))
  (`KismetSystemLibrary.PrintString` (`KismetStringLibrary.Conv_DoubleToString` _health_currentvalue) true true (struct :`G` 0.66 :`B` 1.0 :`A` 1.0) 0.0))

(event `self.SwordCollider.OnComponentBeginOverlap`
  (params (OverlappedComponent :type "PrimitiveComponent Object Reference") (OtherActor :type "Actor Object Reference") (OtherComp :type "PrimitiveComponent Object Reference") (OtherBodyIndex :type Integer) (bFromSweep :type Boolean) (SweepResult :type "HitResult Structure (by ref)"))
  (if (!= OtherActor self)
    (if (== (`GameplayStatics.GetObjectClass` OtherActor) "/Game/Blueprints/Characters/BP_Enemy.BP_Enemy_C")
      (`AbilitySystemBlueprintLibrary.SendGameplayEventToActor` self (struct :`TagName` "skill.melee.dealDamage") (make `GameplayEventData` (struct) null OtherActor)))))

(fn `UserConstructionScript`)