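; Laser beam actor for a gameplay ability that reports hostile characters at the beam's end to its instigator for damage.
; LazerEndDetector overlaps maintain the list of characters hostile to the instigator.
; A looping timer sends that list as target data in a Skill.lazer.dealDamage gameplay event to the instigator.
; Tick stretches the skeletal beam by offsetting its AnimBP end bone to match the detector's distance.
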(event `SendDealDamageEvent`
  ;[1 1 1] Send Damage Event per 0.3 Seconds
  (if (`KismetMathLibrary.Conv_IntToBool` (`KismetArrayLibrary.Array_Length` (`self.OverlappingActors`)))
    _
    (else
      _))
  (`AbilitySystemBlueprintLibrary.SendGameplayEventToActor` (`self.GetInstigator`) (struct :`TagName` "skill.lazer.dealDamage") (make `GameplayEventData` (struct) null null null null (struct) (struct) (struct) 0.0 (`AbilitySystemBlueprintLibrary.AbilityTargetDataFromActorArray` (`self.OverlappingActors`)))))

(event `self.ReceiveBeginPlay`
  (set `self.BeamOriginalLength` (`KismetMathLibrary.VSize` (- (`SceneComponent.GetSocketLocation` (`self.LazerMesh`) "end") (`self.K2_GetActorLocation`))))
  ;[1 1 1] Send Damage Event per 0.3 Seconds
  (`KismetSystemLibrary.K2_SetTimerDelegate` (delegate `SendDealDamageEvent`) 0.3 true))

(event `self.ReceiveTick`
  (params (DeltaSeconds :type "Float (single-precision)"))
  (bind _asanim_bp_lazer_skeletal_mesh_skeleton (cast `/Game/Blueprints/Characters/GameplayAbilities/Lazer/LazerAssets/AnimBP_lazer_skeletal_mesh_Skeleton` (`SkeletalMeshComponent.GetAnimInstance` (`self.LazerMesh`))))
  (set `/Game/Blueprints/Characters/GameplayAbilities/Lazer/LazerAssets/AnimBP_lazer_skeletal_mesh_Skeleton.EndBoneOffset` (`KismetMathLibrary.MakeVector` (- (`KismetMathLibrary.VSize` (- (`SceneComponent.K2_GetComponentLocation` (`self.LazerEndDetector`)) (`self.K2_GetActorLocation`))) (`self.BeamOriginalLength`))) _asanim_bp_lazer_skeletal_mesh_skeleton))

(event `self.LazerEndDetector.OnComponentBeginOverlap`
  (params (OverlappedComponent :type "PrimitiveComponent Object Reference") (OtherActor :type "Actor Object Reference") (OtherComp :type "PrimitiveComponent Object Reference") (OtherBodyIndex :type Integer) (bFromSweep :type Boolean) (SweepResult :type "HitResult Structure (by ref)"))
  (bind _asbp_character_base (cast `/Game/Blueprints/Characters/BP_CharacterBase` OtherActor))
  (bind _asbp_character_base_2 (cast `/Game/Blueprints/Characters/BP_CharacterBase` (`self.GetInstigator`)))
  (bind _returnvalue (`CharacterBase.IsOtherHostile` _asbp_character_base_2 _asbp_character_base))
  (if _returnvalue
    (`KismetArrayLibrary.Array_AddUnique` (`self.OverlappingActors`) _asbp_character_base)))

(event `self.LazerEndDetector.OnComponentEndOverlap`
  (params (OverlappedComponent :type "PrimitiveComponent Object Reference") (OtherActor :type "Actor Object Reference") (OtherComp :type "PrimitiveComponent Object Reference") (OtherBodyIndex :type Integer))
  (bind _asbp_character_base (cast `/Game/Blueprints/Characters/BP_CharacterBase` OtherActor))
  (`KismetArrayLibrary.Array_RemoveItem` (`self.OverlappingActors`) _asbp_character_base))

(fn `UserConstructionScript`)