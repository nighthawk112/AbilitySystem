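; Base Gameplay Ability Blueprint that provides shared helpers for character abilities, leaving activation and end events unimplemented.
; GetPlayerInfo resolves the owning BP_CharacterBase and its BP_PlayerController for the other helpers.
; DoUICooldown starts the cooldown on primary UI slots matching this ability's class.
; IsCostStillAvailable checks whether the Health, Mana or Strength attribute, chosen by cost type, exceeds the negated ability cost.
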(fn `DoUICooldown`
  (bind (_characterbase _playercontroller) (`self.GetPlayerInfo`))
  (`/Engine/EditorBlueprintResources/StandardMacros.IsValid` _playercontroller
    (:`Is Valid`
      (for _array_element (`/Game/UI/PrimaryUI.Slots` (`/Game/Blueprints/BP_PlayerController.Primary UI` _playercontroller))
        (bind _returnvalue (`self.GetAbilityInfo`))
        (bind (_abilityinfo_cooldownduration _abilityinfo_cost _abilityinfo_costtype _abilityinfo_uimat _abilityinfo_abilityclass) (break `GameplayAbilityInfo` (`/Game/UI/WBP_Ability_Slot.AbilityInfo` _array_element)))
        (if (== _abilityinfo_abilityclass (`.AbilityClass` (break `GameplayAbilityInfo` _returnvalue)))
          (`/Game/UI/WBP_Ability_Slot.StartCooldown` _array_element))))))

(fn `GetPlayerInfo`
  (returns (CharacterBase :type "/Game/Blueprints/Characters/BP_CharacterBase Object Reference") (PlayerController :type "/Game/Blueprints/BP_PlayerController Object Reference"))
  (bind _asbp_character_base (cast `/Game/Blueprints/Characters/BP_CharacterBase` (`self.GetOwningActorFromActorInfo`)))
  (bind _asbp_player_controller (cast `/Game/Blueprints/BP_PlayerController` (`Pawn.GetController` _asbp_character_base))
    (:`then`
      _)
    (:`CastFailed`
      _))
  (return _asbp_character_base _asbp_player_controller))

(fn `IsCostStillAvailable`
  (returns (Can :type Boolean))
  (locals (cost :type "Float (double-precision)"))
  (bind _returnvalue (`self.GetAbilityInfo`))
  (set `local.cost` (* (`.Cost` (break `GameplayAbilityInfo` _returnvalue)) -1.0))
  (switch `EAbilityCostType` (`.CostType` (break `GameplayAbilityInfo` _returnvalue))
    (:`Health`
      (bind _characterbase (`self.GetPlayerInfo`))
      (bind (_health_basevalue _health_currentvalue) (break `GameplayAttributeData` (`AttributeSetBase.Health` (`CharacterBase.AttributeSetBaseComp` _characterbase))))
      (return (> _health_currentvalue (`local.cost`))))
    (:`Mana`
      (bind _characterbase_2 (`self.GetPlayerInfo`))
      (bind (_mana_basevalue _mana_currentvalue) (break `GameplayAttributeData` (`AttributeSetBase.Mana` (`CharacterBase.AttributeSetBaseComp` _characterbase_2))))
      (return (> _mana_currentvalue (`local.cost`))))
    (:`Strength`
      (bind _characterbase_3 (`self.GetPlayerInfo`))
      (bind (_strength_basevalue _strength_currentvalue) (break `GameplayAttributeData` (`AttributeSetBase.Strength` (`CharacterBase.AttributeSetBaseComp` _characterbase_3))))
      (return (> _strength_currentvalue (`local.cost`))))))